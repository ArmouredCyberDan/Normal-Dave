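; BP_NPC is a base Blueprint for clickable NPCs that show dialogue in a top-down game.
; OnClick passes the NPC's name and GetDialogue's text, a placeholder for child classes to override, to DisplayDialogue.
; DisplayDialogue enables input on the NPC and has BP_TopDownController create the dialogue, storing the returned widget.
; A left mouse press then calls HideDialogue, handing that widget and the NPC to the controller's EndDialogue.
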(event `Key|LeftMouseButton`
  (params (Key :type "Key Structure"))
  (:`Pressed`
    (`self.HideDialogue`)))

(fn `DisplayDialogue`
  (params (Name :type String) (Dialogue :type String))
  (bind _returnvalue (`GameplayStatics.GetPlayerController` 0))
  (`self.EnableInput` _returnvalue)
  (bind _asbp_top_down_controller (cast `/Game/TopDown/Blueprints/BP_TopDownController` _returnvalue))
  (bind _widget_ref (`/Game/TopDown/Blueprints/BP_TopDownController.InitiateDialogue` _asbp_top_down_controller Name Dialogue))
  (set `self.DialogueWidget` _widget_ref))

(fn `GetDialogue`
  (returns (Dialogue :type String))
  (return "No dialogue! Override the GetDialogue method to manage dialogue."))

(fn `HideDialogue`
  (bind _asbp_top_down_controller (cast `/Game/TopDown/Blueprints/BP_TopDownController` (`GameplayStatics.GetPlayerController` 0)))
  (`/Game/TopDown/Blueprints/BP_TopDownController.End Dialogue` _asbp_top_down_controller (`self.DialogueWidget`) self))

(fn `OnClick`
  (bind _dialogue (`self.GetDialogue`))
  (`self.DisplayDialogue` (`self.Name`) _dialogue))

(fn `UserConstructionScript`
  (`parent.UserConstructionScript`))