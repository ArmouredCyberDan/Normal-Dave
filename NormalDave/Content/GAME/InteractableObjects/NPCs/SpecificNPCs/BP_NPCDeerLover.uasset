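; BP_NPCDeerLover is a specific interactable NPC whose dialogue follows the state of its objective.
; GetDialogue looks up CurrentObjective in the Objectives held by BP_GameInstance_Manager.
; It returns the default Dialogue when the objective is not found, DialogueAfterTalk when it is found but incomplete, and DialogueAfterDead once it is completed.
; The event graph holds only disabled stub events.
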(fn `GetDialogue`
  (returns (Dialogue :type String))
  (bind _currentobjective (`self.CurrentObjective`))
  (bind _asbp_game_instance_manager (cast `/Game/TopDown/Blueprints/BP_GameInstance_Manager` (`GameplayStatics.GetGameInstance`)))
  (if (`.ReturnValue` (`BlueprintMapLibrary.Map_Find` (`/Game/TopDown/Blueprints/BP_GameInstance_Manager.Objectives` _asbp_game_instance_manager) _currentobjective))
    (bind _wascompleted (`/Game/TopDown/Blueprints/BP_GameInstance_Manager.WasObjectiveCompleted` _asbp_game_instance_manager _currentobjective))
    (if _wascompleted
      (return (`self.DialogueAfterDead`))
      (else
        (return (`self.DialogueAfterTalk`))))
    (else
      (return (`self.Dialogue`)))))

(fn `UserConstructionScript`
  (`parent.UserConstructionScript`))