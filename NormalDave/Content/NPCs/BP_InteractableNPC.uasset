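; BP_InteractableNPC is a clickable NPC actor that starts a dialogue with the player.
; On click it enables input on itself, lazily looks up its NPC class in the game instance's NPCs map, and reads its name and dialogue.
; BP_TopDownController opens the dialogue and returns a widget reference, which Space passes back with the actor to end it.
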(event `self.ReceiveActorOnClicked`
  (params (ButtonPressed :type "Key Structure"))
  (bind _returnvalue (`GameplayStatics.GetPlayerController` 0))
  (`self.EnableInput` _returnvalue)
  (`self.SetNPCCLass`)
  (bind (_dialogue _npcname) (`/Game/NPCs/Class_NPC.GetDialogue` (`self.NPCClass`)))
  (bind _asbp_top_down_controller (cast `/Game/TopDown/Blueprints/BP_TopDownController` _returnvalue))
  (bind _widget_ref (`/Game/TopDown/Blueprints/BP_TopDownController.InitiateDialogue` _asbp_top_down_controller _npcname _dialogue))
  (set `self.Widget Ref` _widget_ref))

(event `Key|SpaceBar`
  (params (Key :type "Key Structure"))
  (:`Pressed`
    (bind _asbp_top_down_controller (cast `/Game/TopDown/Blueprints/BP_TopDownController` (`GameplayStatics.GetPlayerController` 0)))
    (`/Game/TopDown/Blueprints/BP_TopDownController.End Dialogue` _asbp_top_down_controller (`self.Widget Ref`) self)))

(fn `SetNPCCLass`
  ;[1 1 1] Check if already set
  (if (== (`self.NPCClass`) null)
    ;[1 1 1] Find in Game Instance and assign
    (bind _asbp_game_instance_manager (cast `/Game/TopDown/Blueprints/BP_GameInstance_Manager` (`GameplayStatics.GetGameInstance`)))
    (set `self.NPCClass` (`BlueprintMapLibrary.Map_Find` (`/Game/TopDown/Blueprints/BP_GameInstance_Manager.NPCs` _asbp_game_instance_manager) (`self.NPC`)))))

(fn `UserConstructionScript`)