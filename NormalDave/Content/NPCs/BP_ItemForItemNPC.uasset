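; BP_ItemForItemNPC is an NPC that trades the player one item for another.
; GetDialogue checks the game instance manager for the accepted item, then completes the objective, swaps the held item for the given one and returns the exchange line.
; If the objective is already done or the player lacks the item, both cases return the same after-exchange dialogue.
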(fn `GetDialogue`
  (returns (Dialogue :type String))
  (bind _wascompleted (`self.WasObjectiveCompleted`))
  (if _wascompleted
    (return (`self.Dialogue_AfterWasGivenItem`))
    (else
      (bind _asbp_game_instance_manager (cast `/Game/TopDown/Blueprints/BP_GameInstance_Manager` (`GameplayStatics.GetGameInstance`)))
      (bind _holdsitem (`/Game/TopDown/Blueprints/BP_GameInstance_Manager.CurrentlyHoldsThisItem` _asbp_game_instance_manager (`self.ItemAccepted`)))
      (if _holdsitem
        (`self.CompleteObjective`)
        (`/Game/TopDown/Blueprints/BP_GameInstance_Manager.ChangeCurrentlyHeldItem` _asbp_game_instance_manager (`self.ItemGiven`))
        (return (`self.Dialogue_WasGivenItem`))
        (else
          (return (`self.Dialogue_AfterWasGivenItem`)))))))

(fn `UserConstructionScript`
  (`parent.UserConstructionScript`))