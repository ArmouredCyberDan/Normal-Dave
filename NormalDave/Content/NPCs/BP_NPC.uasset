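; BP_NPC is a base NPC that shows dialogue when clicked and a tooltip while the cursor hovers over it.
; Clicking enables input on the NPC and has BP_TopDownController open the dialogue widget, which Space closes through the same controller.
; GetDialogue returns placeholder text for child Blueprints to override.
; The construction script applies an optional custom skeletal mesh.
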(event `self.ReceiveActorOnClicked`
  (params (ButtonPressed :type "Key Structure"))
  (bind _dialogue (`self.GetDialogue`))
  (`self.DisplayDialogue` (`self.Name`) _dialogue))

(event `Key|SpaceBar`
  (params (Key :type "Key Structure"))
  (:`Pressed`
    (`self.HideDialogue`)))

(event `self.ReceiveActorBeginCursorOver`
  (bind _uiinstance (`/Game/TopDown/UI/UIFunction.activateUITT` (`KismetTextLibrary.Conv_StringToText` (`self.ToolTip`))))
  (set `self.ToolTipWidget` _uiinstance))

(event `self.ReceiveActorEndCursorOver`
  (`/Game/TopDown/UI/UIFunction.destroyUITT` (`self.ToolTipWidget`)))

(fn `DisplayDialogue`
  (params (Name :type String) (Dialogue :type String))
  (bind _returnvalue (`GameplayStatics.GetPlayerController` 0))
  (`self.EnableInput` _returnvalue)
  (bind _asbp_top_down_controller (cast `/Game/TopDown/Blueprints/BP_TopDownController` _returnvalue))
  (bind _widget_ref (`/Game/TopDown/Blueprints/BP_TopDownController.InitiateDialogue` _asbp_top_down_controller Name Dialogue))
  (set `self.DialogueWidget` _widget_ref))

(fn `GetDialogue`
  (returns (Dialogue :type String))
  (return "No dialogue! Override the GetDialogue method to manage dialogue."))

(fn `HideDialogue`
  (bind _asbp_top_down_controller (cast `/Game/TopDown/Blueprints/BP_TopDownController` (`GameplayStatics.GetPlayerController` 0)))
  (`/Game/TopDown/Blueprints/BP_TopDownController.End Dialogue` _asbp_top_down_controller (`self.DialogueWidget`) self))

(fn `UserConstructionScript`
  (bind _mesh (`self.Mesh`))
  ;[1 1 1] Apply custom mesh if set
  (if (not (== _mesh null))
    (`SkeletalMeshComponent.SetSkeletalMeshAsset` (`self.NPCMesh`) _mesh)))