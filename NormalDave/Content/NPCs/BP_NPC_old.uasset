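; Clickable NPC that shows dialogue through BP_TopDownController and closes it on Space.
; GetDialogue switches on NPC type; only the Futuristic Gang Leader has dialogue logic.
; That logic picks info, item-given or after lines from the GameInstance's GangLeaderGaveItem and CurrentItem, and sets CurrentItem in the after branch.
; The returned Dialogue and Name feed InitiateDialogue crosswise, and the resulting widget is stored for EndDialogue.
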(event `self.ReceiveActorOnClicked`
  (params (ButtonPressed :type "Key Structure"))
  (bind _asbp_top_down_controller (cast `/Game/TopDown/Blueprints/BP_TopDownController` (`GameplayStatics.GetPlayerController` 0)))
  (bind (_dialogue _name) (`self.GetDialogue` (`self.NPC`)))
  (bind _widget_ref (`/Game/TopDown/Blueprints/BP_TopDownController.InitiateDialogue` _asbp_top_down_controller _dialogue _name))
  (set `self.dialoguebox` _widget_ref))

(event `Key|SpaceBar`
  (params (Key :type "Key Structure"))
  (:`Pressed`
    (bind _asbp_top_down_controller (cast `/Game/TopDown/Blueprints/BP_TopDownController` (`GameplayStatics.GetPlayerController` 0)))
    (`/Game/TopDown/Blueprints/BP_TopDownController.End Dialogue` _asbp_top_down_controller (`self.dialoguebox`) null)))

(fn `Dialogue_GangLeader`
  (returns (Dialogue :type String) (Name :type String))
  (locals (InfoDialogue :type String :default "Damn, if only I had the keycard to the secret museum chamber...") (GiveItemDialogue :type String :default "The keycard! Now I can access the secret museum chamber. As a reward, here are some ancient Greek coins!") (AfterDialogue :type String :default "Thank you for the keycard, now I have access to the secret musem chamber."))
  (bind _dialogue_name (`self.Dialogue_Name`))
  (bind _asbp_game_instance_manager (cast `/Game/TopDown/Blueprints/BP_GameInstance_Manager` (`GameplayStatics.GetGameInstance`)))
  (if (`/Game/TopDown/Blueprints/BP_GameInstance_Manager.GangLeaderGaveItem` _asbp_game_instance_manager)
    (set `/Game/TopDown/Blueprints/BP_GameInstance_Manager.GangLeaderGaveItem` true _asbp_game_instance_manager)
    (set `/Game/TopDown/Blueprints/BP_GameInstance_Manager.CurrentItem` "NewEnumerator3" _asbp_game_instance_manager)
    (return (`self.Dialogue_After`) _dialogue_name)
    (elif (`|EnumEquality` (`/Game/TopDown/Blueprints/BP_GameInstance_Manager.CurrentItem` _asbp_game_instance_manager) "NewEnumerator2")
      (return (`self.Dialogue_WasGivenItem`) _dialogue_name)
      (else
        (return (`self.Dialogue_Info`) _dialogue_name)))))

(fn `GetDialogue`
  (params (NPC :type "/Game/NPCs/Enum_NPC Enum" :default "NewEnumerator1"))
  (returns (Dialogue :type String) (Name :type String))
  (switch `/Game/NPCs/Enum_NPC` NPC
    (:`NewEnumerator1`
      _)
    (:`NewEnumerator0`
      (bind (_dialogue _name) (`self.Dialogue_GangLeader`))))
  (return _dialogue _name))

(fn `UserConstructionScript`)