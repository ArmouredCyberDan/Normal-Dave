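; BP_ObjectiveNPC is an NPC Blueprint tied to an objective, exposing functions to complete it and check whether it is done.
; CompleteObjective and WasObjectiveCompleted both cast the game instance to BP_GameInstance_Manager and forward the NPC's Objective variable to it.
; Completion state is read from and written through that game instance manager, and the graphs shown contain no other NPC behavior.
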(fn `CompleteObjective`
  (bind _asbp_game_instance_manager (cast `/Game/TopDown/Blueprints/BP_GameInstance_Manager` (`GameplayStatics.GetGameInstance`)))
  (`/Game/TopDown/Blueprints/BP_GameInstance_Manager.CompleteObjective` _asbp_game_instance_manager (`self.Objective`)))

(fn `UserConstructionScript`
  (`parent.UserConstructionScript`))

(fn `WasObjectiveCompleted`
  (returns (WasCompleted :type Boolean))
  (bind _asbp_game_instance_manager (cast `/Game/TopDown/Blueprints/BP_GameInstance_Manager` (`GameplayStatics.GetGameInstance`)))
  (bind _wascompleted (`/Game/TopDown/Blueprints/BP_GameInstance_Manager.WasObjectiveCompleted` _asbp_game_instance_manager (`self.Objective`)))
  (return _wascompleted))